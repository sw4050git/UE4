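; AI controller for a base NPC that runs BT_NpcBase_Fix and feeds player perception into its blackboard.
; BeginPlay stores the player pawn as PlayerActor and starts the tree.
; Perception updates for Player-tagged actors read stimuli by fixed index: the second sets Flg_Hear and NowDestination, the first drives Flg_Visible.
; Losing that first stimulus starts a timer that clears Flg_Visible after VisibleTimer, giving a grace period that re-detection cancels.
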(event `self.ReceiveBeginPlay`
  ;[1 1 1] BeginPlay
  (`self.UseBlackboard` "/Game/TestGame/Blueprints/Npc/AI/BB_NpcBase.BB_NpcBase")
  (`BlackboardComponent.SetValueAsObject` (`self.Blackboard`) "PlayerActor" (`GameplayStatics.GetPlayerPawn` 0))
  (`self.RunBehaviorTree` "/Game/TestGame/Blueprints/Npc/AI/BT_NpcBase_Fix.BT_NpcBase_Fix"))

(event `self.AIPerception.OnPerceptionUpdated`
  (params (UpdatedActors :type "Array of Actor Object Reference (by ref)"))
  (bind _blackboard (`self.Blackboard`))
  ;[1 1 1] AIPerception
  (for _array_element UpdatedActors
    (if (`self.ActorHasTag` _array_element "Player")
      (bind _info (`AIPerceptionComponent.GetActorsPerception` (`self.AIPerception`) _array_element))
      (`self.UseBlackboard` "/Game/TestGame/Blueprints/Npc/AI/BB_NpcBase.BB_NpcBase")
      (bind (_target _lastsensedstimuli) (break `ActorPerceptionBlueprintInfo` _info))
      (bind (_age _expirationage _strength _stimuluslocation _receiverlocation _tag _bsuccessfullysensed) (break `AIStimulus` (`|GetArrayItem` _lastsensedstimuli 1)))
      (`BlackboardComponent.SetValueAsBool` _blackboard "Flg_Hear" _bsuccessfullysensed)
      (`BlackboardComponent.SetValueAsVector` _blackboard "NowDestination" _stimuluslocation)
      (if (`.bSuccessfullySensed` (break `AIStimulus` (`|GetArrayItem` _lastsensedstimuli)))
        (`KismetSystemLibrary.K2_ClearAndInvalidateTimerHandle` (`self.Timer `))
        (`BlackboardComponent.SetValueAsBool` (`self.Blackboard`) "Flg_Visible" true)
        (else
          (bind _returnvalue (`KismetSystemLibrary.K2_SetTimerDelegate` (delegate `Start Timer`) (`self.Visible Timer`)))
          (set `self.Timer ` _returnvalue)))))
  (set `self.Strength` 0.0))

(event `Start Timer`
  ;[1 1 1] AIPerception
  (`BlackboardComponent.SetValueAsBool` (`self.Blackboard`) "Flg_Visible" false))

(fn `UserConstructionScript`)