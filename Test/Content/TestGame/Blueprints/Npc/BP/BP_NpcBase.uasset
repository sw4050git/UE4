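; Base NPC character that triggers the player's death message on contact.
; When an actor tagged Player overlaps it, the NPC zeroes its walk speed and calls DeadMessage on that actor, passing a point just below the top of its own capsule.
; It also exposes an event to set walk speed and getters for its fixed target point and target points, with no movement logic of its own.
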(event `self.ReceiveBeginPlay`)

(event `self.ReceiveActorBeginOverlap`
  (params (OtherActor :type "Actor Object Reference"))
  (if (`self.ActorHasTag` OtherActor "Player")
    (set `CharacterMovementComponent.MaxWalkSpeed` 0.0 (`self.CharacterMovement`))
    (message `/Game/TestGame/Blueprints/InterFace/BPIF_Player.Dead` OtherActor (`KismetMathLibrary.MakeVector` (.x (`self.K2_GetActorLocation`)) (.y (`self.K2_GetActorLocation`)) (+ (.z (`self.K2_GetActorLocation`)) (- (`CapsuleComponent.GetScaledCapsuleHalfHeight` (`self.CapsuleComponent`)) 20.0))))))

(event `/Game/TestGame/Blueprints/InterFace/BPIF_Npc.UpdateWalkSpeed`
  (params (NewWalkSpeed :type "Float (single-precision)"))
  (set `CharacterMovementComponent.MaxWalkSpeed` NewWalkSpeed (`self.CharacterMovement`)))

(fn `GetFixTargetPoint`
  (returns (FixTargetPoint :type "Actor Object Reference"))
  (return (`self.FixTargetPoint`)))

(fn `GetTargetPoints`
  (returns (TargetPoints :type "Array of Actor Object Reference"))
  (return (`self.TargetPoints`)))

(fn `UserConstructionScript`)