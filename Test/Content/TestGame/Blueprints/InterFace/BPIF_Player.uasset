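; BPIF_Player is a Blueprint Interface that declares the calls other objects can make on the player.
; It covers death with a direction, clear, hiding at a location, peeping, item pickup and consumption, and a memo archive.
; Getters expose the target actor, widget, forward vector and heart rate, which has a setter taking a new panic rate.
; The functions are signatures only, so implementers supply all behavior.
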(fn `AddMemoArchive`
  (params (MemoTitle :type Text) (Memo :type Text)))

(fn `Clear`)

(fn `ConsumeItem`)

(fn `Dead`
  (params (Direction :type "Vector Structure"))
  (return))

(fn `GetForwardVector`
  (returns (ForwardVector :type "Vector Structure"))
  (return (0.0 0.0 0.0)))

(fn `GetHeartRate`
  (returns (HeartRate :type "Float (double-precision)"))
  (return 0.0))

(fn `GetMemoArchive`
  (returns (MemoArchive :type "Array of /Game/TestGame/Blueprints/Structures/ST_MemoArchive Structure"))
  (return))

(fn `GetTargetActor`
  (returns (TargetActor :type "Actor Object Reference"))
  (return null))

(fn `GetWidget`
  (returns (Widget :type "UserWidget Object Reference"))
  (return null))

(fn `Hide`
  (params (Location :type "Vector Structure"))
  (returns (Hiding :type Boolean))
  (return false))

(fn `Peep`
  (returns (Peeping :type Boolean))
  (return false))

(fn `Pickup`
  (params (ItemData :type "/Game/TestGame/Blueprints/Objects/Items/BP_ItemDataAsset Object Reference") (Num :type Integer))
  (returns (Successed :type Boolean))
  (return false))

(fn `SetHeartRate`
  (params (NewPanicRate :type "Float (double-precision)")))