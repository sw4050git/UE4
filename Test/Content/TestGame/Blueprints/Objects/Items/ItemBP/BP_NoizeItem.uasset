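; BP_NoizeItem is a usable item that throws a noise source from the player.
; ItemUse spawns a BP_NoiseSource at the player's transform and applies a forward-and-upward impulse to its Body, using the player's forward vector.
; It then tells the player to consume the item through a message call and destroys itself.
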(event `/Game/TestGame/Blueprints/InterFace/BPIF_ItemUse.ItemUse`
  (params (Player :type "Actor Object Reference"))
  (bind _forwardvector (message `/Game/TestGame/Blueprints/InterFace/BPIF_Player.GetForwardVector` Player))
  (bind _returnvalue (`|SpawnActorFromClass` "/Game/TestGame/Blueprints/Objects/Items/BP_NoiseSource.BP_NoiseSource_C" (`self.GetTransform` Player) "Undefined" "OverrideRootScale" null null))
  (`PrimitiveComponent.AddImpulse` (`/Game/TestGame/Blueprints/Objects/Items/BP_NoiseSource.Body` _returnvalue) (* (`KismetMathLibrary.MakeVector` (.x _forwardvector) (.y _forwardvector) (+ (.z _forwardvector) 1.0)) 500.0) "None" false)
  (message `/Game/TestGame/Blueprints/InterFace/BPIF_Player.ConsumeItem` Player)
  (`self.K2_DestroyActor`))

(fn `UserConstructionScript`
  (`parent.UserConstructionScript`))