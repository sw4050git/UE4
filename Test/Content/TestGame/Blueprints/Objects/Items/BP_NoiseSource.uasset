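; BP_NoiseSource is a temporary item actor that emits AI-perceivable noise during a timed window.
; BeginPlay chains delays to keep tick off at first, enable it briefly, disable it again, then destroy the actor.
; While ticking, it reports a noise event every frame at the Body component's location, using Loudness as both loudness and max range.
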(event `self.ReceiveBeginPlay`
  (`self.SetActorTickEnabled` false)
  (`KismetSystemLibrary.Delay` 5.0)
  (`self.SetActorTickEnabled` true)
  (`KismetSystemLibrary.Delay` 5.0)
  (`self.SetActorTickEnabled` false)
  (`KismetSystemLibrary.Delay` 10.0)
  (`self.K2_DestroyActor`))

(event `self.ReceiveTick`
  (params (DeltaSeconds :type "Float (single-precision)"))
  (bind _loudness (`self.Loudness`))
  (`AISense_Hearing.ReportNoiseEvent` (`SceneComponent.K2_GetComponentLocation` (`self.Body`)) _loudness self _loudness))

(fn `UserConstructionScript`)